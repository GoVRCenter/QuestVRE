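; BP_Terminal_Master_Main is a terminal Blueprint that colors itself by its Team: Red, Blue or Friendly.
; The Construction Script creates a dynamic material instance on the static mesh and stores it as MID.
; It then selects the team color, saves it to Color and applies it to both point lights.
; The material's LightColor parameter receives the same color at half intensity.
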(fn `UserConstructionScript`
  (bind _staticmesh (`self.StaticMesh`))
  (bind _mid (`self.MID`))
  (bind _color (`self.Color`))
  (bind _pointlight (`self.PointLight`))
  (bind (_red _blue _friendly) (break `/Game/Blueprints/DATA/TeamColors` (`|Copy` (struct))))
  (bind _returnvalue (`KismetMathLibrary.Conv_ColorToLinearColor` _red))
  (bind _returnvalue_2 (`KismetMathLibrary.Conv_ColorToLinearColor` _friendly))
  (bind _returnvalue_3 (`KismetMathLibrary.Conv_ColorToLinearColor` _blue))
  (bind _returnvalue_4 (`PrimitiveComponent.CreateDynamicMaterialInstance` _staticmesh 0 null "None"))
  (bind _output_get (set `self.MID` _returnvalue_4))
  (`PrimitiveComponent.SetMaterial` _staticmesh 0 _output_get)
  (switch `/Game/Blueprints/DATA/Enum_Teams` (`self.Team`)
    (:`NewEnumerator0`
      (`KismetMathLibrary.LinearColor_Set` _color _returnvalue)
      (`LightComponent.SetLightColor` _pointlight _returnvalue true)
      (`LightComponent.SetLightColor` (`self.PointLight1`) _returnvalue true)
      (`MaterialInstanceDynamic.SetVectorParameterValue` _mid "LightColor" (* _returnvalue 0.5)))
    (:`NewEnumerator1`
      (`KismetMathLibrary.LinearColor_Set` _color _returnvalue_3)
      (`LightComponent.SetLightColor` _pointlight _returnvalue_3 true)
      (`LightComponent.SetLightColor` (`self.PointLight1`) _returnvalue_3 true)
      (`MaterialInstanceDynamic.SetVectorParameterValue` _mid "LightColor" (* _returnvalue_3 0.5)))
    (:`NewEnumerator2`
      (`KismetMathLibrary.LinearColor_Set` _color _returnvalue_2)
      (`LightComponent.SetLightColor` _pointlight _returnvalue_2 true)
      (`LightComponent.SetLightColor` (`self.PointLight1`) _returnvalue_2 true)
      (`MaterialInstanceDynamic.SetVectorParameterValue` _mid "LightColor" (* _returnvalue_2 0.5)))))