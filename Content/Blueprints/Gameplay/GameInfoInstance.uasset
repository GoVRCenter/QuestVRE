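; Game instance Blueprint that handles multiplayer session hosting and joining, plus a save-slot existence check for player settings.
; LaunchLobby stores the match settings, destroys any old session, creates a new one and opens the Lobby level as a listen server.
; JoinServer likewise clears the old session first, continuing even if that fails.
; Network and travel error handlers print converted messages, though both converter functions currently return empty strings.
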(event `SaveGameCheck`
  ;[1 1 1] Check for a save Game Slot Name
  (bind _returnvalue (`GameplayStatics.DoesSaveGameExist` (`self.Save_PlayerSettings`)))
  (bind _output_get (set `self.HasSaveGame` _returnvalue))
  (if _output_get
    _))

(event `LaunchLobby`
  (params (NumberOfPlayers :type Integer) (IsLAN :type Boolean) (ServerName :type Text) (SelectedMap :type Integer) (PlayToScore :type Integer))
  (bind _returnvalue (`GameplayStatics.GetPlayerController` 0))
  ;[1 1 1] Launch Lobby
  (bind _output_get (set `self.MaxNumOfPlayers` NumberOfPlayers))
  (set `self.SelectedMap` SelectedMap)
  (set `self.PlayToScore` PlayToScore)
  (set `self.ServerName` ServerName)
  (`DestroySessionCallbackProxy.DestroySession` _returnvalue
    (:`OnSuccess`
      _)
    (:`OnFailure`
      _))
  (`CreateSessionCallbackProxy.CreateSession` _returnvalue _output_get IsLAN
    (:`OnSuccess`
      (`GameplayStatics.OpenLevel` "Lobby" true "listen"))
    (:`OnFailure`
      (`KismetSystemLibrary.PrintString` "Failed to create server session"))))

(event `JoinServer`
  (params (SessionToJoin :type "BlueprintSessionResult Structure"))
  (bind _returnvalue (`GameplayStatics.GetPlayerController` 0))
  ;[1 1 1] Join Server
  (`DestroySessionCallbackProxy.DestroySession` _returnvalue
    (:`OnSuccess`
      _)
    (:`OnFailure`
      _))
  (`JoinSessionCallbackProxy.JoinSession` _returnvalue SessionToJoin
    (:`then`
      (`KismetSystemLibrary.PrintString` "Joining selected Server..." true true (struct :`G` 0.66 :`B` 1.0 :`A` 1.0) 6.0))
    (:`OnSuccess`
      (`KismetSystemLibrary.PrintString` "REPORTED  Success Joining listen Server" true true (struct :`G` 0.66 :`B` 1.0 :`A` 1.0) 6.0))
    (:`OnFailure`
      (`KismetSystemLibrary.PrintString` "Failed to join session" true true (struct :`G` 0.66 :`B` 1.0 :`A` 1.0) 6.0))))

(event `self.HandleNetworkError`
  (params (FailureType :type "ENetworkFailure Enum" :default "NetDriverAlreadyExists") (bIsServer :type Boolean))
  ;[1 1 1] Network Errors
  (if bIsServer
    _
    (else
      _))
  (`KismetSystemLibrary.PrintString` (`self.NetworkErrorToString` FailureType)))

(event `self.HandleTravelError`
  (params (FailureType :type "ETravelFailure Enum" :default "NoLevel"))
  ;[1 1 1] Network Errors
  (`KismetSystemLibrary.PrintString` (`self.TravelErrorToString` FailureType)))

(event `DestroySessionCaller`
  (params (PlayerController :type "PlayerController Object Reference"))
  ;[1 1 1] End Old Session
  (`DestroySessionCallbackProxy.DestroySession` PlayerController))

(fn `NetworkErrorToString`
  (params (FailureType :type "ENetworkFailure Enum" :default "NetDriverAlreadyExists"))
  (returns (OutSTring :type String))
  (return ""))

(fn `TravelErrorToString`
  (params (FailureType :type "ETravelFailure Enum" :default "NoLevel"))
  (returns (OutString :type String))
  (return ""))